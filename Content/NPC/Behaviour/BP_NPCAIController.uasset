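; AI controller for guard NPCs that starts the patrol blackboard and guard behavior tree on BeginPlay.
; Perception updates feed the blackboard: sight stores the sensed actor as the player, while other senses store its current location as last known.
; Any failed stimulus clears the player key, and every update prints debug text.
; Aim-pitch and player-cast logic remain unconnected.
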(event `self.ReceiveBeginPlay`
  (bind _blackboardcomponent (`self.UseBlackboard` "/Game/NPC/Behaviour/PatrolData.PatrolData"))
  (set `self.BlackboardComp` _blackboardcomponent)
  (`self.RunBehaviorTree` "/Game/NPC/Behaviour/GuardBehaviour.GuardBehaviour"))

(event `self.AIPerception.OnTargetPerceptionUpdated`
  (params (Actor :type "Actor Object Reference") (Stimulus :type "AIStimulus Structure"))
  (bind _blackboardcomp (`self.BlackboardComp`))
  (bind _playerkeyname (`self.PlayerKeyName`))
  (`self.PrintPerceptionDebug` Actor Stimulus)
  (if (`.bSuccessfullySensed` (break `AIStimulus` Stimulus))
    (bind _returnvalue (`AIPerceptionSystem.GetSenseClassForStimulus` Stimulus))
    (if (== _returnvalue "/Script/AIModule.AISense_Sight")
      (`BlackboardComponent.SetValueAsObject` _blackboardcomp _playerkeyname Actor)
      (else
        (`BlackboardComponent.SetValueAsVector` _blackboardcomp (`self.LastKnownLocationKey`) (`self.K2_GetActorLocation` Actor))))
    (else
      (`BlackboardComponent.ClearValue` _blackboardcomp _playerkeyname))))

(fn `PrintPerceptionDebug`
  (params (Actor :type "Object Object Reference") (StimulusClass :type "AIStimulus Structure"))
  (bind _returnvalue (`AIPerceptionSystem.GetSenseClassForStimulus` StimulusClass))
  (`KismetSystemLibrary.PrintString` (`KismetStringLibrary.Concat_StrStr` (`KismetSystemLibrary.GetDisplayName` (`self.K2_GetPawn`)) " " (`KismetSystemLibrary.GetClassDisplayName` _returnvalue) " " (`KismetSystemLibrary.GetDisplayName` Actor))))

(fn `UserConstructionScript`)